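; Pause menu controller that toggles game pause and drives the PauseMenuWidget through Enhanced Input.
; On BeginPlay it finds the 3Cats player and its controller, adds the IMC_Menu mapping context and creates the widget.
; Menu actions toggle pause, scroll the widget and confirm selections while paused.
; SetPause switches input mode, cursor, widget visibility, game pause and player input together.
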(event Input|EnhancedActionEvents|EnhancedInputActionIA_MenuPause
  (params (ActionValue :type Boolean) (ElapsedSeconds :type Float%20%28double-precision%29) (TriggeredSeconds :type Float%20%28double-precision%29) (InputAction :type Input%20Action%20Object%20Reference :default "/Game/ThirdPerson/Input/IA_MenuPause.IA_MenuPause"))
  (:Started
    (CallFunction|SetPause (not (Game|IsGamePaused)))))

(event Input|EnhancedActionEvents|EnhancedInputActionIA_MenuNavigate
  (params (ActionValue :type Float%20%28double-precision%29) (ElapsedSeconds :type Float%20%28double-precision%29) (TriggeredSeconds :type Float%20%28double-precision%29) (InputAction :type Input%20Action%20Object%20Reference :default "/Game/ThirdPerson/Input/IA_MenuNavigate.IA_MenuNavigate"))
  (:Triggered
    (Default|Scroll (Variables|Default|GetPauseMenuWidget) (> ActionValue 0.0))))

(event Input|EnhancedActionEvents|EnhancedInputActionIA_MenuConfirm
  (params (ActionValue :type Boolean) (ElapsedSeconds :type Float%20%28double-precision%29) (TriggeredSeconds :type Float%20%28double-precision%29) (InputAction :type Input%20Action%20Object%20Reference :default "/Game/ThirdPerson/Input/IA_MenuConfirm.IA_MenuConfirm"))
  (:Triggered
    (if (Game|IsGamePaused) :!label _label
      (Default|Confirm (Variables|Default|GetPauseMenuWidget))))
  (:Started
    (goto _label)))

(event EventBeginPlay
  (bind _returnvalue (Actor|GetActorOfClass "/Game/ThirdPerson/Blueprints/3Cats.3Cats_C"))
  (bind _asplayer_controller (Utilities|Casting|CastToPlayerController (Pawn|GetController (Variables|/Script/Engine.Actor|GetInstigator _returnvalue))))
  (bind _output_get (Variables|Default|SetAs%20Player%20Controller _asplayer_controller))
  (Utilities|IsValid (PlayerController|LocalPlayerSubsystems|GetEnhancedInputLocalPlayerSubsystem _output_get)
    (:Is%20Valid
      (Input|AddMappingContext (PlayerController|LocalPlayerSubsystems|GetEnhancedInputLocalPlayerSubsystem _output_get) "/Game/ThirdPerson/Input/IMC_Menu.IMC_Menu" 0 "(bIgnoreAllPressedKeysUntilRelease=True,bForceImmediately=False)")
      (bind _returnvalue_2 (UserInterface|CreateWidget "/Game/Blueprints/PauseMenuWidget.PauseMenuWidget_C"))
      (bind _output_get_2 (Variables|Default|SetPauseMenuWidget _returnvalue_2))
      (UserInterface|Viewport|AddtoViewport _output_get_2 0)
      (Variables|/Game/Blueprints/PauseMenuWidget.PauseMenuWidget_C|SetPauseMenu _output_get_2 self)
      (bind _returnvalue_3 (Actor|GetActorOfClass "/Game/ThirdPerson/Blueprints/3Cats.3Cats_C"))
      (Variables|Default|SetPlayer _returnvalue_3))))

(fn ConstructionScript)

(fn SetPause
  (params (State :type Boolean))
  (bind _as_player_controller (Variables|Default|GetAs%20Player%20Controller))
  (bind _pausemenuwidget (Variables|Default|GetPauseMenuWidget))
  (if State
    (Input|SetInputModeGameandUI _as_player_controller _pausemenuwidget "DoNotLock" true false)
    (else
      (Input|SetInputModeGameOnly _as_player_controller false)))
  (Variables|/Script/Engine.PlayerController|SetbShowMouseCursor _as_player_controller State)
  (Default|Hide _pausemenuwidget State)
  (Game|SetGamePaused State)
  (Default|ToggleInput (Variables|Default|GetPlayer) State)
  (Variables|Default|SetLock false))