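; WaterSpill is a spill actor that makes overlapping 3Cats characters slide.
; WaterExpand plays the Test timeline, which lerps the Water component's X and Y scale to grow the puddle, while Nowater stops it.
; Water's begin and end overlap events switch sliding on and off through ToggleSliding on the character.
; Disconnected nodes that set ground friction and braking deceleration directly remain in the graph unused.
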(event OnComponentBeginOverlap(Water)
  (params (OverlappedComponent :type Primitive%20Component%20Object%20Reference) (OtherActor :type Actor%20Object%20Reference) (OtherComp :type Primitive%20Component%20Object%20Reference) (OtherBodyIndex :type Integer) (bFromSweep :type Boolean) (SweepResult :type Hit%20Result%20Structure%20%28by%20ref%29))
  (bind _as3cats (Utilities|Casting|CastTo3Cats OtherActor))
  (Default|ToggleSliding _as3cats true))

(event OnComponentEndOverlap(Water)
  (params (OverlappedComponent :type Primitive%20Component%20Object%20Reference) (OtherActor :type Actor%20Object%20Reference) (OtherComp :type Primitive%20Component%20Object%20Reference) (OtherBodyIndex :type Integer))
  (bind _as3cats (Utilities|Casting|CastTo3Cats OtherActor))
  (Default|ToggleSliding _as3cats false))

(event Custom|WaterExpand
  (bind _newtrack_0 (Timeline|test Play)
    (:Update
      (Transformation|SetRelativeScale3D (Variables|Default|GetWater) (Math|Vector|MakeVector (Math|Float|Lerp 0.1 3e+01 _newtrack_0) (Math|Float|Lerp 0.1 3e+01 _newtrack_0) 1.0)))))

(event Custom|Nowater
  (bind _newtrack_0 (Timeline|test Stop)
    (:Update
      (Transformation|SetRelativeScale3D (Variables|Default|GetWater) (Math|Vector|MakeVector (Math|Float|Lerp 0.1 3e+01 _newtrack_0) (Math|Float|Lerp 0.1 3e+01 _newtrack_0) 1.0)))))

(event EventBeginPlay)

(event Collision|EventActorBeginOverlap
  (params (OtherActor :type Actor%20Object%20Reference)))

(fn ConstructionScript)