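; DrinkLever is a lever actor that operates a drink machine and a linked light.
; Each tick it reads the lever's pitch in actor-local space and treats a negative angle as on.
; Any change of state, in either direction, calls Lightuse on the LightSwitch, then DrinkSpawn on the DrinkMachine.
; Without a valid LightSwitch it resets to off and spawns nothing; its Use function is empty.
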(event EventBeginPlay)

(event Collision|EventActorBeginOverlap
  (params (OtherActor :type Actor%20Object%20Reference)))

(event EventTick
  (params (DeltaSeconds :type Float%20%28single-precision%29))
  (bind _returnvalue (Transformation|GetActorTransform))
  (bind _lever (Variables|Components|GetLever))
  (bind _returnvalue_2 (Transformation|GetWorldRotation _lever))
  (bind _returnvalue_3 (Math|Transform|InverseTransformRotation _returnvalue _returnvalue_2))
  (bind _pitch (Math|Rotator|BreakRotator _returnvalue_3))
  (bind _returnvalue_4 (< _pitch 0.0))
  (if (!= (Variables|Default|GetOn) _returnvalue_4)
    (Variables|Default|SetOn _returnvalue_4)
    (bind _aslight_switch (Utilities|Casting|CastToLightSwitch (Variables|Default|GetLight))
      (:then
        (Default|Lightuse _aslight_switch)
        (bind _asdrink_machine (Utilities|Casting|CastToDrinkMachine (Variables|Default|GetDrink)))
        (Default|DrinkSpawn _asdrink_machine))
      (:CastFailed
        (Variables|Default|SetOn false)))))

(fn ConstructionScript)

(fn Use)