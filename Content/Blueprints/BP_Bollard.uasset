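; BP_Bollard is a roped bollard barrier that breaks when the 3Cats actor runs into it.
; On overlap with BlockerNorth, it waits briefly, randomly detaches the start or end of the Cable, then destroys that blocker.
; BeginPlay caches the 3Cats actor, but the logic that would toggle north and south blocker collision by which side it is on is disconnected and never runs.
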(event OnComponentBeginOverlap(BlockerNorth)
  (params (OverlappedComponent :type Primitive%20Component%20Object%20Reference) (OtherActor :type Actor%20Object%20Reference) (OtherComp :type Primitive%20Component%20Object%20Reference) (OtherBodyIndex :type Integer) (bFromSweep :type Boolean) (SweepResult :type Hit%20Result%20Structure%20%28by%20ref%29))
  (bind _cable (Variables|Default|GetCable))
  (Utilities|Casting|CastTo3Cats OtherActor)
  (Utilities|FlowControl|Delay 0.2)
  (switch int (Math|Random|RandomInteger 2)
    (:0
      (Variables|/Script/CableComponent.CableComponent|SetbAttachEnd _cable false))
    (:1
      (Variables|/Script/CableComponent.CableComponent|SetbAttachStart _cable false)))
  (Components|DestroyComponent (Variables|Default|GetBlockerNorth)))

(event EventBeginPlay
  (bind _returnvalue (Actor|GetActorOfClass "/Game/ThirdPerson/Blueprints/3Cats.3Cats_C"))
  (Variables|Default|SetNewVar _returnvalue))

(event Collision|EventActorBeginOverlap
  (params (OtherActor :type Actor%20Object%20Reference)))

(event EventTick
  (params (DeltaSeconds :type Float%20%28single-precision%29)))

(fn ConstructionScript)