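; Drink machine Blueprint that toggles a water stream and drives a linked WaterSpill.
; Water starts hidden at BeginPlay, and each DrinkSpawn event flips the SpawnDrink flag.
; A true flag hides Water and calls Nowater on the spill, while false shows Water and calls WaterExpand.
; A separate Drinkgone event only clears the Destroy flag.
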(event Custom|Drinkgone
  (Variables|Default|Setdestroy false))

(event Custom|DrinkSpawn
  (Variables|Default|SetSpawnDrink (!= (Variables|Default|GetSpawnDrink) true))
  (if (Variables|Default|GetSpawnDrink)
    (Development|SetHiddeninGame (Variables|Default|GetWater) true false)
    (bind _aswater_spill (Utilities|Casting|CastToWaterSpill (Variables|Default|GetwaterSpill)))
    (Default|Nowater _aswater_spill)
    (else
      (Development|SetHiddeninGame (Variables|Default|GetWater) false false)
      (bind _aswater_spill_2 (Utilities|Casting|CastToWaterSpill (Variables|Default|GetwaterSpill)))
      (Default|WaterExpand _aswater_spill_2))))

(event Collision|EventActorBeginOverlap
  (params (OtherActor :type Actor%20Object%20Reference)))

(event EventTick
  (params (DeltaSeconds :type Float%20%28single-precision%29)))

(event EventBeginPlay
  (Development|SetHiddeninGame (Variables|Default|GetWater) true false))

(fn ConstructionScript)