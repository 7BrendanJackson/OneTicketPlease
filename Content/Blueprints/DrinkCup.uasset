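; Drink cup that shows liquid rising by scaling its Drink component on the Z axis.
; Tick plays the FullCup timeline while CupGettingDrink is true and stops it otherwise, with the WaterFilling track driving the scale.
; FillCup toggles that flag, while StopCup assigns it its own value through a not-equal-false comparison, so it leaves the state unchanged.
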(event Custom|FillCup
  (Variables|Default|SetCupGettingDrink (!= (Variables|Default|GetCupGettingDrink) true)))

(event Custom|StopCup
  (Variables|Default|SetCupGettingDrink (!= (Variables|Default|GetCupGettingDrink) false)))

(event EventBeginPlay)

(event Collision|EventActorBeginOverlap
  (params (OtherActor :type Actor%20Object%20Reference)))

(event EventTick
  (params (DeltaSeconds :type Float%20%28single-precision%29))
  (if (Variables|Default|GetCupGettingDrink)
    (bind _waterfilling (Timeline|FullCup Play)
      (:Update
        (Transformation|SetRelativeScale3D (Variables|Default|GetDrink) (Math|Vector|MakeVector 1.0 1.0 (Math|Float|Lerp 0.0 0.2 _waterfilling)))))
    (else
      (Timeline|FullCup Stop))))

(fn ConstructionScript)