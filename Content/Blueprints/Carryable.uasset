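; Carryable item that the 3Cats actor can pick up and throw.
; OnUse disables the Cube's physics and collision, attaches it to the "carry" socket with tunable offsets, stops sparkles and plays a sound.
; Drop restores physics, calls AttachActorToActor without a parent, and applies forward ThrowForce.
; Both update CarriedItem after a short delay; Drop also delays restoring pawn blocking and sparkles.
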(event Custom|Drop
  (bind _3cats (Variables|Default|Get3Cats))
  (Collision|SetCollisionEnabled (Variables|Default|GetCube) "QueryAndPhysics")
  (Transformation|AttachActorToActor 0 "None" "KeepRelative" "KeepRelative" "KeepRelative" true)
  (Physics|SetSimulatePhysics (Variables|Default|GetCube) true)
  (Physics|AddForce (Variables|Default|GetCube) (* (Transformation|GetActorForwardVector _3cats) (Variables|Default|GetThrowForce)) "None" true)
  (Utilities|FlowControl|Delay 0.2)
  (Variables|/Game/ThirdPerson/Blueprints/3Cats.3Cats_C|SetCarriedItem _3cats 0)
  (Collision|SetCollisionResponsetoChannel (Variables|Default|GetCube) "ECC_Pawn" "ECR_Block")
  (Components|Activation|Activate (Variables|Default|GetSparkles) false))

(event EventBeginPlay
  (bind _returnvalue (Actor|GetActorOfClass "/Game/ThirdPerson/Blueprints/3Cats.3Cats_C"))
  (bind _output_get (Variables|Default|Set3Cats _returnvalue)))

(event Collision|EventActorBeginOverlap
  (params (OtherActor :type Actor%20Object%20Reference)))

(event EventTick
  (params (DeltaSeconds :type Float%20%28single-precision%29)))

(event EventOnUse
  (Physics|SetSimulatePhysics (Variables|Default|GetCube) false)
  (Collision|SetCollisionEnabled (Variables|Default|GetCube) "NoCollision")
  (Collision|SetCollisionResponsetoChannel (Variables|Default|GetCube) "ECC_Pawn" "ECR_Ignore")
  (Transformation|AttachComponentToComponent (Variables|/Script/Engine.Character|GetMesh (stale EventBeginPlay _output_get)) "carry" "SnapToTarget" "SnapToTarget" "KeepWorld" true)
  (Transformation|AddActorLocalOffset (Variables|Default|GetoffsetPosition) false true)
  (Transformation|AddActorLocalRotation (Variables|Default|GetoffsetRotation) false false)
  (Components|Activation|Deactivate (Variables|Default|GetSparkles))
  (Audio|PlaySoundatLocation "/Game/Audio/Other_Sounds/PickUpItem.PickUpItem" (Transformation|GetActorLocation (Variables|Default|Get3Cats)) "0, 0, 0" 1.0 1.0 0.0 0 0 0 0)
  (Utilities|FlowControl|Delay 0.2)
  (Variables|/Game/ThirdPerson/Blueprints/3Cats.3Cats_C|SetCarriedItem (Variables|Default|Get3Cats) self))

(fn ConstructionScript)

(fn NewFunction)

(fn DropSelf)