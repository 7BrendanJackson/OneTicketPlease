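; BP_GrindRail is a grind rail actor that builds its visible track along a spline; no grinding movement is implemented here.
; The construction script tiles spline mesh segments by the mesh's X bounds, clamping tangents to segment length and applying a material.
; Each segment binds a begin-overlap event.
; The overlap handler only unbinds actor overlap events and prints a debug message for actors lacking BPI_Player.
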(event EventBeginPlay)

(event Collision|EventActorBeginOverlap
  (params (OtherActor :type Actor%20Object%20Reference)))

(event EventTick
  (params (DeltaSeconds :type Float%20%28single-precision%29)))

(fn ConstructionScript
  (bind _mesh (Variables|Default|GetMesh))
  (bind _spline (Variables|Default|GetSpline))
  (bind _spline_2 (Variables|Default|GetSpline))
  (bind _returnvalue (StaticMesh|GetBoundingBox _mesh))
  (bind _output_get (Variables|Default|SetXLength (.x (+ (Math|Vector|VectorGetAbs (.min _returnvalue)) (Math|Vector|VectorGetAbs (.max _returnvalue))))))
  (for _index (range 0 (Math|Float|Truncate (/ (Spline|GetSplineLength (Variables|Default|GetSpline)) _output_get)))
    (bind _returnvalue_2 (AddComponent|AddSplineMeshComponent false))
    (Collision|BindEventtoOnComponentBeginOverlap _returnvalue_2 (EventDispatchers|CreateEvent :!event BPGrindRailAutoGenFunc))
    (bind _output_get_2 (Variables|Default|SetSplineMesh _returnvalue_2))
    (Components|StaticMesh|SetStaticMesh _output_get_2 (Variables|Default|GetMesh))
    (SplineMesh|SetStartandEnd _output_get_2 (Spline|GetLocationatDistanceAlongSpline _spline_2 (* _index (Variables|Default|GetXLength)) "Local") (Math|Vector|ClampVectorSize (Spline|GetTangentatDistanceAlongSpline _spline_2 (* _index (Variables|Default|GetXLength)) "Local") 0.0 (Variables|Default|GetXLength)) (Spline|GetLocationatDistanceAlongSpline _spline (* (+ _index 1) (Variables|Default|GetXLength)) "Local") (Math|Vector|ClampVectorSize (Spline|GetTangentatDistanceAlongSpline _spline (* (+ _index 1) (Variables|Default|GetXLength)) "Local") 0.0 (Variables|Default|GetXLength)) true :!class /Script/Engine.SplineMeshComponent)
    (Rendering|Material|SetMaterial _output_get_2 0 (Variables|Default|GetMaterial))))

(fn BPGrindRailAutoGenFunc
  (params (OverlappedComponent :type Primitive%20Component%20Object%20Reference) (OtherActor :type Actor%20Object%20Reference) (OtherComp :type Primitive%20Component%20Object%20Reference) (OtherBodyIndex :type Integer) (bFromSweep :type Boolean) (SweepResult :type Hit%20Result%20Structure%20%28by%20ref%29))
  (if (not (Utilities|DoesObjectImplementInterface OtherActor "/Game/BPI_Player.BPI_Player_C"))
    (EventDispatchers|UnbindallEventsfromOnActorBeginOverlap)
    (Development|PrintString (Utilities|String|Append "Added to Grindrail: " (Utilities|GetDisplayName OtherActor)))
    (return)))